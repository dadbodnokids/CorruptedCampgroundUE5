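; Hex grid board actor that lays out flat-top tiles as instances of one mesh in an InstancedStaticMesh.
; The construction script measures the mesh bounds at the chosen scale, then loops over Height and Width to place instances using hex spacing plus an Offset gap.
; A FlipFlop after each row toggles a negative small-radius X shift, staggering alternate rows into a honeycomb.
; The event graph has no active logic.
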(event EventBeginPlay)

(event Collision|EventActorBeginOverlap
  (params (OtherActor :type Actor%20Object%20Reference)))

(event EventTick
  (params (DeltaSeconds :type Float%20%28single-precision%29)))

(fn ConstructionScript
  (Components|StaticMesh|SetStaticMesh (Variables|Default|GetInstancedStaticMesh) (Variables|Components|GetTileMesh))
  (CallFunction|CalculateSizes)
  (for _index (range 0 (Variables|Integers|GetHeight))
    (bind _returnvalue (CallFunction|HorizontalSpace _index))
    (for _index_2 (range 0 (Variables|Integers|GetWidth))
      (bind _returnvalue_2 (CallFunction|VerticalSpace _index_2))
      (Components|InstancedStaticMesh|AddInstance (Variables|Default|GetInstancedStaticMesh) (Math|Transform|MakeTransform (Math|Vector|MakeVector (+ _returnvalue_2 (Variables|Floats|GetRowOffset)) _returnvalue 0.0) "0, 0, 0" (Math|Conversions|ToVector(Float) (Variables|Floats|GetScale))) false))
    (Utilities|FlowControl|FlipFlop
      (:A
        (CallFunction|OffsetHexagons))
      (:B
        (Variables|Floats|SetRowOffset 0.0)))))

(fn CalculateSizes
  (bind _tilemesh (Variables|Components|GetTileMesh))
  (bind _scale (Variables|Floats|GetScale))
  (bind _returnvalue (StaticMesh|GetBoundingBox _tilemesh))
  (bind _output_get (Variables|Floats|SetRadiusSmall (* (.x (.max _returnvalue)) _scale)))
  (Variables|Floats|SetDiameterSmall (* _output_get 2.0))
  (bind _output_get_2 (Variables|Floats|SetRadiusLarge (* (.y (.max _returnvalue)) _scale)))
  (Variables|Floats|SetDiameterLarge (* _output_get_2 2.0)))

(fn VerticalSpace
  (params (HexNum :type Integer))
  (return (+ (* HexNum (Variables|Floats|GetOffset)) (* HexNum (Math|Float|Sqrt 3.0) (Variables|Floats|GetRadiusLarge)))))

(fn HorizontalSpace
  (params (HexNum :type Integer))
  (return (+ (* HexNum (Variables|Floats|GetOffset)) (* HexNum (Variables|Floats|GetDiameterLarge) 0.75))))

(fn OffsetHexagons
  (Variables|Floats|SetRowOffset (* (Variables|Floats|GetRadiusSmall) -1.0)))