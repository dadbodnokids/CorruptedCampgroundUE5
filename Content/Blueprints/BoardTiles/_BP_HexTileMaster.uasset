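; Master Blueprint for a clickable hex board tile that serves as a movement target for player pieces.
; The construction script sets the mesh material from TileType: grass, path or water.
; Clicking the collision component calls MovePlayerToTile on every BP_PlayerPiece actor, passing the tile mesh's X/Y, a fixed height and a movement cost of one regardless of tile type.
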(event OnClicked(Collision)
  (params (TouchedComponent :type Primitive%20Component%20Object%20Reference) (ButtonPressed :type Key%20Structure :default "None"))
  (bind _staticmesh (Variables|Default|GetStaticMesh))
  (bind _returnvalue (Transformation|GetWorldLocation _staticmesh))
  (Development|PrintString "Tile Clicked")
  (bind _outactors (Actor|GetAllActorsOfClass "/Game/Blueprints/Character/BP_PlayerPiece.BP_PlayerPiece_C"))
  (for _array_element _outactors
    (bind _output_get (Variables|Default|SetPlayerReference _array_element))
    (Default|MovePlayertoTile _output_get (Math|Vector|MakeVector (.x _returnvalue) (.y _returnvalue) 21.0) 1 false)))

(event EventBeginPlay)

(event Collision|EventActorBeginOverlap
  (params (OtherActor :type Actor%20Object%20Reference)))

(event EventTick
  (params (DeltaSeconds :type Float%20%28single-precision%29)))

(fn ConstructionScript
  (bind _staticmesh (Variables|Default|GetStaticMesh))
  (switch Utilities|FlowControl|Switch|SwitchonE_TileType (Variables|Default|GetTileType)
    (:NewEnumerator0
      (Rendering|Material|SetMaterial _staticmesh 0 (Variables|Materials|GetGrassMaterial)))
    (:NewEnumerator1
      (Rendering|Material|SetMaterial _staticmesh 0 (Variables|Materials|GetPathMaterial)))
    (:NewEnumerator2
      (Rendering|Material|SetMaterial _staticmesh 0 (Variables|Materials|GetWaterMaterial)))))