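; Player piece Blueprint that moves between tiles and spends action points.
; MovePlayerToTile requires CanPlayerMove and a non-obstacle tile, calls CalculatePlayerActionPoints, then sets the actor to TileLocation's X and Y at a fixed height.
; The cost is deducted only when ActionPoints cover it, but the move happens either way.
; Print strings report remaining points after deduction and each move.
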(event Custom|MovePlayerToTile
  (params (TileLocation :type Vector) (MovementCost :type Integer) (bIsObstacle? :type Boolean))
  (if (Variables|Default|GetbCanPlayerMove?)
    (if (not bIsObstacle?)
      (CallFunction|CalculatePlayerActionPoints MovementCost MovementCost)
      (Transformation|SetActorLocation (Math|Vector|MakeVector (.x TileLocation) (.y TileLocation) 21.0) false false)
      (Development|PrintString "Player Moved"))))

(event EventBeginPlay)

(event Collision|EventActorBeginOverlap
  (params (OtherActor :type Actor%20Object%20Reference)))

(event EventTick
  (params (DeltaSeconds :type Float%20%28single-precision%29)))

(fn ConstructionScript)

(fn CalculatePlayerActionPoints
  (params (MovementAP :type Integer) (CurrentAP :type Integer))
  (if (<= CurrentAP (Variables|Default|GetActionPoints))
    (Variables|Default|SetActionPoints (- (Variables|Default|GetActionPoints) MovementAP))
    (Development|PrintString (Utilities|String|ToString(Integer) (Variables|Default|GetActionPoints)))))